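; Base enemy character Blueprint that handles the death sequence with a dissolve effect.
; OnEnemyDead pauses animation, disables capsule collision and async-loads the supplied Niagara system to attach to the mesh, tinting it from the material's dissolve edge color.
; A timeline scaled to TotalDissolveTime drives DissolveAmount on the body and equipped weapon, then destroys both.
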(event EventBeginPlay)

(event Collision|EventActorBeginOverlap
  (params (OtherActor :type Actor%20Object%20Reference)))

(event EventTick
  (params (DeltaSeconds :type Float%20%28single-precision%29)))

(event EventOnEnemyDead
  (params (DissolveNiagaraSystem :type Niagara%20System%20Soft%20Object%20Reference))
  (Utilities|FlowControl|Sequence
    (:then_0
      (Variables|/Script/Engine.SkeletalMeshComponent|SetbPauseAnims (Variables|Character|GetMesh) true)
      (Collision|SetCollisionEnabled (Variables|Default|GetCapsuleComponent) "NoCollision"))
    (:then_1
      (bind _object (Utilities|AsyncLoadAsset DissolveNiagaraSystem)
        (:Completed
          (bind _asniagara_system (Utilities|Casting|CastToNiagaraSystem _object))
          (bind _returnvalue (Niagara|SpawnSystemAttached _asniagara_system (Variables|Character|GetMesh) "None" "0, 0, 0" "0, 0, 0" "KeepRelativeOffset" true))
          (CallFunction|SetDissolveParticleColor _returnvalue)
          (Components|Timeline|SetPlayRate (Variables|Default|GetDissolveTimeline) (/ 1.0 (Variables|Default|GetTotalDissolveTime)))
          (bind _dissolvetrack (Timeline|DissolveTimeline PlayFromStart)
            (:Update
              (CallFunction|SetDissolveMaterial _dissolvetrack))
            (:Finished
              (CallFunction|DestoryActorandWeapon))))))))

(fn ConstructionScript)

(fn DestoryActorandWeapon
  (bind _enemycombatcomponent (Variables|Default|GetEnemyCombatComponent))
  (bind _returnvalue (Class|PawnCombatComponent|GetCharacterCurrentEquippedWeapon _enemycombatcomponent))
  (Utilities|IsValid _returnvalue
    (:Is%20Valid
      (Actor|DestroyActor _returnvalue))
    (:Is%20Not%20Valid
      _))
  (Actor|DestroyActor))

(fn SetDissolveMaterial
  (params (DissolveTrack :type Float%20%28single-precision%29))
  (bind _enemycombatcomponent (Variables|Default|GetEnemyCombatComponent))
  (bind _returnvalue (Class|PawnCombatComponent|GetCharacterCurrentEquippedWeapon _enemycombatcomponent))
  (Rendering|Material|SetScalarParameterValueonMaterials (Variables|Character|GetMesh) "DissolveAmount" DissolveTrack)
  (Utilities|IsValid _returnvalue
    (:Is%20Valid
      (Rendering|Material|SetScalarParameterValueonMaterials (Variables|/Script/Kloto.KlotoWeaponBase|GetWeaponMesh _returnvalue) "DissolveAmount" DissolveTrack))))

(fn SetDissolveParticleColor
  (params (NiagaraSystem :type Niagara%20Component%20Object%20Reference))
  (bind _mesh (Variables|Character|GetMesh))
  (bind _returnvalue (Rendering|Material|CreateDynamicMaterialInstance _mesh 0 (Rendering|Material|GetMaterial _mesh 0) "None" :!class /Script/Engine.PrimitiveComponent))
  (bind _returnvalue_2 (Rendering|Material|GetVectorParameterValue _returnvalue "DissolveEdgeColor" :!class /Script/Engine.MaterialInstanceDynamic))
  (Niagara|SetNiagaraVariable(LinearColor) NiagaraSystem "DissolveParticleColor" _returnvalue_2))