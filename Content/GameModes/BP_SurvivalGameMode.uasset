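; Survival game mode Blueprint that announces wave progress on screen as the survival state changes.
; BeginPlay binds OnSurvivalGameModeChanged, whose handler switches on state to show wave text widgets, with countdowns for waiting and completed waves.
; The final wave also sets the enemy spawn delay and shows a delayed "Last Wave" banner.
; All-waves-done and player-death states only print debug strings; wave spawning logic is not in this graph.
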(event Custom|OnSurvivalGameModeChanged_Event
  (params (CurrentState :type EKlotoSurvivalGameModeState%20Enum :default "WaitSpawnNewWave"))
  (switch Utilities|FlowControl|Switch|SwitchonEKlotoSurvivalGameModeState CurrentState
    (:WaitSpawnNewWave
      (CallFunction|CreateWaveWidgetwithCountDown "New Wave Coming In" (Variables|Default|GetSpawnNewWaveWaitTime)))
    (:SpawningNewWave
      (CallFunction|CreateWaveWidgetNoCountDown (Utilities|Text|FormatText "Wave {WaveCount} " (Variables|Default|GetCurrentWaveCount)))
      (if (== (Variables|Default|GetCurrentWaveCount) (Variables|Default|GetTotalWavesToSpawn))
        (Variables|Default|SetSpawnEnemiesDelayTime 4.0)
        (Utilities|FlowControl|Delay 2.0)
        (CallFunction|CreateWaveWidgetNoCountDown "Last Wave")))
    (:WaveCompleted
      (CallFunction|CreateWaveWidgetwithCountDown (Utilities|Text|FormatText "Wave {WaveCount} Completed" (Variables|Default|GetCurrentWaveCount)) (Variables|Default|GetWaveCompletedWaitTime)))
    (:AllWavesDone
      (Development|PrintString "All Waves Done" true true "(R=0.000000,G=0.660000,B=1.000000,A=1.000000)" 8.0))
    (:PlayerDied
      (Development|PrintString "Player Died" true true "(R=0.000000,G=0.660000,B=1.000000,A=1.000000)" 8.0))))

(event EventBeginPlay
  (EventDispatchers|AssignOnSurvivalGameModeChanged (delegate Custom|OnSurvivalGameModeChanged_Event)))

(event EventTick
  (params (DeltaSeconds :type Float%20%28single-precision%29)))

(fn ConstructionScript)

(fn CreateWaveWidgetwithCountDown
  (params (TextContentToDisplay :type Text) (InTotalCountDownTime :type Float%20%28double-precision%29))
  (bind _returnvalue (UserInterface|CreateWidget "/Game/Widgets/GameModeWidgets/WBP_WaveTextWithCountDown.WBP_WaveTextWithCountDown_C"))
  (bind _output_get (LocalVariables|SetWBP_WaveTextWithCountDown _returnvalue))
  (UserInterface|Viewport|AddtoViewport _output_get 0)
  (Rendering|Components|TextRender|SetText (Variables|/Game/Widgets/GameModeWidgets/WBP_WaveTextWithCountDown.WBP_WaveTextWithCountDown_C|GetTextBlock_NewWave (LocalVariables|GetWBP_WaveTextWithCountDown)) TextContentToDisplay)
  (Default|StartCountDown (LocalVariables|GetWBP_WaveTextWithCountDown) InTotalCountDownTime))

(fn CreateWaveWidgetNoCountDown
  (params (TextContentToDisplay :type Text))
  (bind _returnvalue (UserInterface|CreateWidget "/Game/Widgets/GameModeWidgets/WBP_WaveTextNoCountDown.WBP_WaveTextNoCountDown_C"))
  (bind _output_get (LocalVariables|SetWBP_WaveTextNoCountDown _returnvalue))
  (UserInterface|Viewport|AddtoViewport _output_get 0)
  (Rendering|Components|TextRender|SetText (Variables|/Game/Widgets/GameModeWidgets/WBP_WaveTextNoCountDown.WBP_WaveTextNoCountDown_C|GetTextBlock_NewWave (LocalVariables|GetWBP_WaveTextNoCountDown)) TextContentToDisplay))